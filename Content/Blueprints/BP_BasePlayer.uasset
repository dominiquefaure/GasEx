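; Base player Blueprint that sets up the HUD and starting sword when play begins.
; It creates and displays WBP_HUD, spawns BP_Sword and equips it in the PrimaryWeapon slot through EquipmentManager.
; The sword's hit component is then registered with GxCombat as the MainWeapon source.
; A test input draws a short debug line trace along the mesh's forward vector; the sprint toggle input is unimplemented.
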(event `self.ReceiveBeginPlay`
  (`self.InitHUD`)
  (bind _returnvalue (`|SpawnActorFromClass` "/Game/Blueprints/Weapons/BP_Sword.BP_Sword_C" (`KismetMathLibrary.MakeTransform` (0.0 0.0 0.0)) "Undefined" "MultiplyWithRoot" null null))
  (`EquipmentManagerComponent.EquipItem` (`self.EquipmentManager`) "PrimaryWeapon" _returnvalue)
  (bind _asbp_sword (cast `/Game/Blueprints/Weapons/BP_Sword` _returnvalue))
  (bind _returnvalue_2 (`WeaponActor.GetHitComponent` _asbp_sword))
  (`/Engine/EditorBlueprintResources/StandardMacros.IsValid` _returnvalue_2
    (:`Is Valid`
      (`GxCombatComponent.RegisterHitComponent` (`self.GxCombat`) "MainWeapon" _returnvalue_2))))

(event `EnhancedInput|/Game/Input/Actions/IA_SprintToggle`
  (params (ActionValue :type Boolean) (ElapsedSeconds :type "Float (double-precision)") (TriggeredSeconds :type "Float (double-precision)") (InputAction :type "InputAction Object Reference" :default "/Game/Input/Actions/IA_SprintToggle.IA_SprintToggle")))

(event `EnhancedInput|/Game/Input/Actions/IA_Test`
  (params (ActionValue :type Boolean) (ElapsedSeconds :type "Float (double-precision)") (TriggeredSeconds :type "Float (double-precision)") (InputAction :type "InputAction Object Reference" :default "/Game/Input/Actions/IA_Test.IA_Test"))
  (bind _returnvalue_location (`KismetMathLibrary.BreakTransform` (`self.GetTransform`)))
  (:`Triggered`
    (`KismetSystemLibrary.LineTraceSingle` :`Start` _returnvalue_location :`End` (+ _returnvalue_location (* (`KismetMathLibrary.GetForwardVector` (`SceneComponent.K2_GetComponentRotation` (`self.Mesh`))) 200.0)) :`TraceChannel` "TraceTypeQuery1" :`DrawDebugType` "ForDuration")))

(fn `InitHUD`
  (bind _returnvalue (`|CreateWidget` "/Game/UI/WBP_HUD.WBP_HUD_C"))
  (bind _output_get (set `self.HUD` _returnvalue))
  (`UserWidget.AddToViewport` _output_get 0))

(fn `UserConstructionScript`)