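; Burn Knuckle gameplay ability, a special attack that dashes the owning actor forward with a dashing cross animation.
; On activation it commits, plays the montage and starts a root motion move-to force toward a point a short distance straight ahead.
; The ability ends when the move finishes or the montage completes or is interrupted, and cancels if the montage is cancelled.
; Ending the ability also ends the montage task.
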(event `self.K2_ActivateAbility`
  (bind _returnvalue (`self.GetOwningActorFromActorInfo`))
  (`self.K2_CommitAbility`)
  (bind _asynctaskproxy (`AbilityTask_PlayMontageAndWait.CreatePlayMontageAndWaitProxy` "None" "/Game/Art/Characters/Mannequins/Animations/Attacks/SpecialAttacks/Crunch_Ability_DashingCross_Montage.Crunch_Ability_DashingCross_Montage" 1.0 "None" true 1.0 0.0 true)
    (:`then`
      (set `self.PlayMontageTask` _asynctaskproxy)
      (`AbilityTask_ApplyRootMotionMoveToForce.ApplyRootMotionMoveToForce` "None" (+ (`Actor.K2_GetActorLocation` _returnvalue) (* (`Actor.GetActorForwardVector` _returnvalue) 300.0)) 3.0 false "MOVE_None" false null "MaintainLastRootMotionVelocity"
        (:`OnTimedOutAndDestinationReached`
          (`self.K2_EndAbility`))))
    (:`OnCompleted`
      (`self.K2_EndAbility` :!label _label))
    (:`OnInterrupted`
      (goto _label))
    (:`OnCancelled`
      (`self.K2_CancelAbility`))))

(event `self.K2_OnEndAbility`
  (params (bWasCancelled :type Boolean))
  (`GameplayTask.EndTask` (`self.PlayMontageTask`)))